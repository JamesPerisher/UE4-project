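; Door Blueprint that plays a Level Sequence when any actor overlaps it, presumably to open and close the door.
; Begin and end overlap set the Intrigger flag and share one branch that plays NewLevelSequence forward on entry and in reverse on exit.
; Each overlap change creates a new sequence player rather than reusing one.
; BeginPlay only runs a Delay with nothing after it.
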(event EventBeginPlay
  (Utilities|FlowControl|Delay 2.0))

(event EventTick
  (params (DeltaSeconds :type Float%20%28single-precision%29)))

(event Collision|EventActorBeginOverlap
  (params (OtherActor :type Actor%20Object%20Reference))
  (Variables|Default|Setintrigger true)
  (if (Variables|Default|Getintrigger)
    (bind _returnvalue (Sequencer|Player|CreateLevelSequencePlayer "/Game/LevelSequences/NewLevelSequence.NewLevelSequence"))
    (Sequencer|Player|Play _returnvalue :!class /Script/MovieScene.MovieSceneSequencePlayer)
    (else
      (bind _returnvalue_2 (Sequencer|Player|CreateLevelSequencePlayer "/Game/LevelSequences/NewLevelSequence.NewLevelSequence"))
      (Class|MovieSceneSequencePlayer|PlayReverse _returnvalue_2))))

(event Collision|EventActorEndOverlap
  (params (OtherActor :type Actor%20Object%20Reference))
  (Variables|Default|Setintrigger false)
  (if (Variables|Default|Getintrigger)
    (bind _returnvalue (Sequencer|Player|CreateLevelSequencePlayer "/Game/LevelSequences/NewLevelSequence.NewLevelSequence"))
    (Sequencer|Player|Play _returnvalue :!class /Script/MovieScene.MovieSceneSequencePlayer)
    (else
      (bind _returnvalue_2 (Sequencer|Player|CreateLevelSequencePlayer "/Game/LevelSequences/NewLevelSequence.NewLevelSequence"))
      (Class|MovieSceneSequencePlayer|PlayReverse _returnvalue_2))))

(fn ConstructionScript)