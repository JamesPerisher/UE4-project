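; Inventory component that holds a fixed-size array of item slots, sized on BeginPlay, and toggles an inventory window.
; Adding items tops up a partial stack of the same class, or writes them into the first empty slot if none exists.
; Overflow beyond max stack size is fed back recursively through AddtoInventory.
; The toggle creates or removes a centre-anchored widget on the player controller's HUD canvas, switching between UI-only and game-only input.
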(event EventBeginPlay
  (CallFunction|PrepairInventory))

(fn ToggleInventory
  (bind _inventorywindow (Variables|Default|GetInventoryWindow)
    (:then
      ;[1 1 1] Delete Render
      (Widget|RemovefromParent _inventorywindow)
      (Variables|Default|SetInventoryWindow 0)
      (Input|SetInputModeGameOnly (Game|GetPlayerController 0)))
    (:else
      ;[1 1 1] Render Position inventory
      (bind _returnvalue (UserInterface|CreateWidget "/Game/Blueprints/InventorySystem/InventoryUI/InventoryWindow.InventoryWindow_C" 0 self))
      (Variables|Default|SetInventoryWindow _returnvalue)
      (bind _ascustom_player_controller (Utilities|Casting|CastToCustomPlayerController (Game|GetPlayerController 0)))
      (bind _returnvalue_2 (Class|CanvasPanel|AddChildtoCanvas (Variables|/Game/Blueprints/InventorySystem/InventoryUI/InventoryHud.InventoryHud_C|GetHudCanvas (Variables|/Game/Blueprints/CustomPlayerController.CustomPlayerController_C|GetHudWidget _ascustom_player_controller)) (Variables|Default|GetInventoryWindow)))
      (Class|CanvasPanelSlot|SetAutoSize _returnvalue_2 true)
      (Class|CanvasPanelSlot|SetAlignment _returnvalue_2 "(X=0.500000,Y=0.500000)")
      (Class|CanvasPanelSlot|SetAnchors _returnvalue_2 (Utilities|Struct|MakeAnchors "(X=0.500000,Y=0.500000)" "(X=0.500000,Y=0.500000)"))
      (Class|CanvasPanelSlot|SetPosition _returnvalue_2 (Variables|Default|GetPosition))
      (Input|SetInputModeUIOnly (Game|GetPlayerController 0) (Variables|Default|GetInventoryWindow) "LockAlways"))))

(fn AddtoInventory
  (params (ContentsToAdd :type Slot%20Structure%20Structure))
  ;[1 1 1] Add to Stack if existing else make new stack
  (bind _stackindex (Utilities|HasPartialStack ContentsToAdd)
    (:True
      (CallFunction|AddtoStack ContentsToAdd _stackindex))
    (:False
      (CallFunction|CreateStack ContentsToAdd)))
  (return true))

(fn PrepairInventory
  (Utilities|Array|Resize (Variables|Default|GetInventory) (Variables|Default|GetNumberOfSlots))
  (return))

(fn CreateStack
  (params (ContentsToAdd :type Slot%20Structure%20Structure))
  (bind _inventory (Variables|Default|GetInventory))
  ;[1 1 1] find next empty slot and add to it
  (Utilities|Array|SetArrayElem _inventory (Utilities|Array|FindItem _inventory (Utilities|Struct|MakeSlotStructure "(Name_6_32D4BB8C499FC86FDA6970A0A25E3AC0=NSLOCTEXT(\"[A8D11A2D4952B28E396F29BAADDF1265]\", \"BA64988E4F66A21DFB2CD8978813BEEA\", \"Item\"),Hover_5_7B39625942CD76666A2848902D708C10=NSLOCTEXT(\"[A8D11A2D4952B28E396F29BAADDF1265]\", \"C74DEC3149BCCCAED56FD6BE4CB08597\", \"Description\"),Maxstack_9_2EA328214A1B7329C4C07D9ED410A569=-1,Icon_12_ED3700B14837A45BFA2FF590184733BE=None,Durability_15_033D8FD14C00D6D108AD9580BA4AFD58=1.000000,Class_21_D6B830184F8D9F5A98F395B2FAEC39FF=None)")) ContentsToAdd))

(fn AddtoStack
  (params (SlotStructure :type Slot%20Structure%20Structure) (Index :type Integer))
  (bind _inventory (Variables|Default|GetInventory))
  (bind _inventory_2 (Variables|Default|GetInventory))
  (bind _maxstack (Utilities|Struct|BreakItemStructure (.itemstructure SlotStructure)))
  (bind _output (Utilities|Array|Get(acopy) _inventory Index))
  (bind _output_2 (Utilities|Array|Get(acopy) _inventory_2 Index))
  ;[1 1 1] True if exiting stack > max stack
  (bind _output_get (LocalVariables|SetCurrentQuantity (.quantaty _output)))
  (if (> (+ _output_get (.Quantaty (Utilities|Struct|BreakSlotStructure SlotStructure))) (.maxstack (.itemstructure _output)))
    ;[1 1 1] exiting + toadd > max stack fill to max
    (Utilities|Array|SetArrayElem (Variables|Default|GetInventory) Index (Utilities|Struct|MakeSlotStructure (.itemstructure SlotStructure) _maxstack))
    ;[1 1 1] add leftover again
    (CallFunction|AddtoInventory (Utilities|Struct|MakeSlotStructure (.itemstructure SlotStructure) (- (.quantaty SlotStructure) (- _maxstack (LocalVariables|GetCurrentQuantity)))))
    (else
      ;[1 1 1] All good add to stack count
      (Utilities|Array|SetArrayElem _inventory_2 Index (Utilities|Struct|MakeSlotStructure (.itemstructure _output_2) (+ (.quantaty _output_2) (.quantaty SlotStructure))))))
  (return))