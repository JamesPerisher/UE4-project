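; Interactable sound-test actor that plays its assigned sound when used.
; The Interact event plays the sound wave from its Sound component's SoundWaveParam at the actor's location.
; The construction script writes that sound's display name to two text render components, so each placed instance labels itself in the editor.
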(event EventInteract
  (params (Interactor :type Actor%20Object%20Reference))
  ;[1 1 1] play sound on interact
  (Audio|PlaySoundatLocation (.soundwaveparam (Variables|Default|GetSound)) (.location (Transformation|GetActorTransform)) "0, 0, 0" 1.0 1.0 0.0 0 0 0))

(fn ConstructionScript
  ;[1 1 1] set Text based on soundfilename
  (Variables|Default|Settext (Utilities|Text|ToText(String) (Utilities|GetDisplayName (.soundwaveparam (Variables|Default|GetSound)))))
  (Rendering|Components|TextRender|SetText (Variables|Default|GetTextRender) (Variables|Default|Gettext))
  (Rendering|Components|TextRender|SetText (Variables|Default|GetTextRender1) (Variables|Default|Gettext)))